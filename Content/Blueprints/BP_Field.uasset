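; BP_Field is a 2D stage field that builds itself to a configurable length in the Construction Script.
; It lays out one Paper2D field sprite per stage part, spaced by StageLength along X.
; BoxTop and BoxBottom are stretched and centred to span all parts.
; GoalTop and GoalBottom are offset from their current X toward the far end, StageEndBeforeMapFinish parts short of the full length.
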(event EventBeginPlay)

(event Collision|EventActorBeginOverlap
  (params (OtherActor :type Actor%20Object%20Reference)))

(event EventTick
  (params (DeltaSeconds :type Float%20%28single-precision%29)))

(fn ConstructionScript
  ;[1 0.25 0.25] Loop for all stage parts, if we have more stage would be bigger
  (for _index (range 0 (- (Variables|Default|GetStageParts) 1))
    ;[0.2791 0.3676 1] This is getting the sprite and will be creating one, using the stage length as muiplyer with index
    (bind _returnvalue (AddComponent|AddPaperSpriteComponent false (Math|Transform|MakeTransform (Math|Vector|MakeVector (Math|Conversions|ToFloat(Integer) (* _index (Variables|Default|GetStageLength))) 0.0 0.0) "0, 0, 0" "1.000000,1.000000,1.000000")))
    (Rendering|Components|Sprite|SetSprite _returnvalue "/Game/PaperAssets/Background/T_Field_Sprite.T_Field_Sprite"))
  ;[1 0.3191 0.06708] Creating the map extension through the game, setting the box and the etent from box top to box bottom
  (CallFunction|UpdateBoxExtent (Variables|Default|GetBox%20Top))
  (CallFunction|UpdateBoxExtent (Variables|Default|GetBoxBottom))
  (CallFunction|UpdateBoxLocation (Variables|Default|GetBox%20Top))
  (CallFunction|UpdateBoxLocation (Variables|Default|GetBoxBottom))
  ;[0.3695 0.9202 1] Getting current position plus multiplier to the stage lenght to build the end of the game TOP
  (CallFunction|UpdateGoalLocation (Variables|Default|GetGoalTop))
  ;[0.3695 0.9202 1] Getting current position plus multiplier to the stage lenght to build the end of the game BOTTOM
  (CallFunction|UpdateGoalLocation (Variables|Default|GetGoalBottom)))

(fn UpdateBoxExtent
  (params (Box :type Box%20Component%20Object%20Reference))
  (bind _boxextent (Variables|/Script/Engine.BoxComponent|GetBoxExtent Box))
  (Components|Box|SetBoxExtent Box (Math|Vector|MakeVector (Math|Conversions|ToFloat(Integer) (* (/ (Variables|Default|GetStageLength) 2) (Variables|Default|GetStageParts))) (.y _boxextent) (.z _boxextent)) true))

(fn UpdateBoxLocation
  (params (Box :type Scene%20Component%20Object%20Reference))
  (bind _relativelocation (Variables|/Script/Engine.SceneComponent|GetRelativeLocation Box))
  (Transformation|SetRelativeLocation Box (Math|Vector|MakeVector (Math|Conversions|ToFloat(Integer) (- (/ (* (Variables|Default|GetStageLength) (Variables|Default|GetStageParts)) 2) (/ (Variables|Default|GetStageLength) 2))) (.y _relativelocation) (.z _relativelocation)) false false))

(fn UpdateGoalLocation
  (params (Goal :type Scene%20Component%20Object%20Reference))
  (bind _relativelocation (Variables|/Script/Engine.SceneComponent|GetRelativeLocation Goal))
  (Transformation|SetRelativeLocation Goal (Math|Vector|MakeVector (+ (* (- (Variables|Default|GetStageParts) (Variables|Default|GetStageEndBeforeMapFinish)) (Variables|Default|GetStageLength)) (.x _relativelocation)) (.y _relativelocation) (.z _relativelocation)) false false))