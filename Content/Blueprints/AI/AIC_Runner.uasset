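; AI controller for BP_Runner that drives the pawn by simulating player input.
; On possess it caches the runner, and on BeginPlay it schedules the first simulated input.
; A FlipFlop alternates left and right power calls on the runner, rescheduling a one-shot timer with a random delay between the min and max input delays after each.
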(event Custom|SimulateInput
  ;[0.2153 0.7448 0.2952] This is to simulate the input
  (Utilities|FlowControl|FlipFlop
    (:A
      (Default|SimulatePowerLeft (Variables|Default|GetOwningRunner))
      (CallFunction|SimulateInputwithDelay))
    (:B
      (Default|SimulatePowerRight (Variables|Default|GetOwningRunner))
      (CallFunction|SimulateInputwithDelay))))

(event EventBeginPlay
  ;[0.1264 1 0.1388] Begin play
  (CallFunction|SimulateInputwithDelay))

(event EventPossess
  (params (PossessedPawn :type Pawn%20Object%20Reference))
  ;[1 0.2292 0.2292] This will trigger only once at the begining of the AI object
  (bind _asbp_runner (Utilities|Casting|CastToBP_Runner PossessedPawn))
  (Variables|Default|SetOwningRunner _asbp_runner))

(fn ConstructionScript)

(fn SimulateInputwithDelay
  (Utilities|Time|SetTimerbyEvent (EventDispatchers|CreateEvent :!event Custom|SimulateInput) (Math|Random|RandomFloatinRange (Variables|Default|GetMinInputDelay) (Variables|Default|GetMaxInputDelay))))