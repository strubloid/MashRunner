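; Player runner character with a flipbook sprite, driven by alternating left and right taps to build speed.
; Each valid alternate tap raises max walk speed through a velocity-based ramp, while Tick decays it and constantly applies forward movement along X.
; Distance and speed feed an on-screen widget.
; Velocity selects the idle or run flipbook and scales run playback, with footstep sounds keyed to specific frames.
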(event Input|EnhancedActionEvents|EnhancedInputActionAI_PowerLeft
  (params (ActionValue :type Boolean) (ElapsedSeconds :type Float%20%28double-precision%29) (TriggeredSeconds :type Float%20%28double-precision%29) (InputAction :type Input%20Action%20Object%20Reference :default "/Game/Input/Actions/AI_PowerLeft.AI_PowerLeft"))
  (:Started
    ;[1 0.5089 0.3684] Increasing speed if is correct the sequence
    (bind _speedreturned (CallFunction|IncreaseSpeedRule "NewEnumerator1" "NewEnumerator1"))
    ;[1 1 1] Casting to Background options
    (bind _aswid_background_options (Utilities|Casting|CastToWID_Background_Options (Variables|Default|GetWID_CharacterSpeed)))
    (Default|UpdateData _aswid_background_options (.x (Class|CharacterMovementComponent|GetLastUpdateLocation (Variables|/Script/Engine.Character|GetCharacterMovement (Game|GetPlayerCharacter 0)))) _speedreturned)))

(event Input|EnhancedActionEvents|EnhancedInputActionAI_PowerRight
  (params (ActionValue :type Boolean) (ElapsedSeconds :type Float%20%28double-precision%29) (TriggeredSeconds :type Float%20%28double-precision%29) (InputAction :type Input%20Action%20Object%20Reference :default "/Game/Input/Actions/AI_PowerRight.AI_PowerRight"))
  (:Started
    ;[1 0.5089 0.3684] Increasing speed if is correct the sequence
    (bind _speedreturned (CallFunction|IncreaseSpeedRule "NewEnumerator2" "NewEnumerator2"))
    ;[1 1 1] Casting to Background options
    (bind _aswid_background_options (Utilities|Casting|CastToWID_Background_Options (Variables|Default|GetWID_CharacterSpeed)))
    (Default|UpdateData _aswid_background_options (.x (Class|CharacterMovementComponent|GetLastUpdateLocation (Variables|/Script/Engine.Character|GetCharacterMovement (Game|GetPlayerCharacter 0)))) _speedreturned)))

(event EventBeginPlay
  (bind _asplayer_controller (Utilities|Casting|CastToPlayerController (Pawn|GetController)))
  (Input|AddMappingContext (PlayerController|LocalPlayerSubsystems|GetEnhancedInputLocalPlayerSubsystem _asplayer_controller) "/Game/Input/IMC_Runner.IMC_Runner" 0 "(bIgnoreAllPressedKeysUntilRelease=True,bForceImmediately=False,bNotifyUserSettings=False)")
  (bind _returnvalue (UserInterface|CreateWidget "/Game/Blueprints/WID_Background_Options.WID_Background_Options_C" (Game|GetPlayerController 0)))
  (bind _output_get (Variables|Default|SetWID_CharacterSpeed _returnvalue))
  (UserInterface|Viewport|AddtoViewport _output_get 0))

(event Collision|EventActorBeginOverlap
  (params (OtherActor :type Actor%20Object%20Reference)))

(event EventTick
  (params (DeltaSeconds :type Float%20%28single-precision%29))
  (Pawn|Input|AddMovementInput "1.000000,0.000000,0.000000" 1.0 false)
  (bind _speed (CallFunction|DecreaseSpeed DeltaSeconds))
  (bind _returnvalue_x (CallFunction|GetCurrentDistance))
  (Default|UpdateData (Variables|Default|GetWID_CharacterSpeed) _returnvalue_x _speed)
  (CallFunction|UpdateFlipbook)
  (CallFunction|SetRunPlayRate)
  (CallFunction|StepsSound))

(fn ConstructionScript)

(fn IncreaseSpeed
  (bind _output_get (Variables|/Script/Engine.CharacterMovementComponent|SetMaxWalkSpeed (Variables|Character|GetCharacterMovement) (Math|Float|Clamp(Float) (+ (Variables|/Script/Engine.CharacterMovementComponent|GetMaxWalkSpeed (Variables|Character|GetCharacterMovement)) (* (Variables|Default|GetSpeedIncreasePerTap) (Math|Curves|GetFloatValue (Variables|Default|GetSpeedIncreaseRamp) (Math|Vector|VectorLength (Variables|/Script/Engine.MovementComponent|GetVelocity (Variables|Character|GetCharacterMovement)))))) 0.0 (Variables|Default|GetMaxSpeed))))
  (return _output_get))

(fn IncreaseSpeedRule
  (params (Cond1 :type E_Input%20Enum :default "NewEnumerator0") (Cond2 :type E_Input%20Enum :default "NewEnumerator0"))
  (if (Utilities|Enum|NotEqual(Enum) (Variables|Default|GetLastInput) Cond1)
    (Variables|Default|SetLastInput Cond2)
    (bind _speedreturned (CallFunction|IncreaseSpeed))
    (bind _output_get (LocalVariables|SetLastSpeedReturned _speedreturned))
    (return _output_get)
    (else
      (return (LocalVariables|GetLastSpeedReturned)))))

(fn DecreaseSpeed
  (params (DeltaSeconds :type Float%20%28single-precision%29))
  (bind _output_get (Variables|/Script/Engine.CharacterMovementComponent|SetMaxWalkSpeed (Variables|Character|GetCharacterMovement) (Math|Float|Max(Float) (- (Variables|/Script/Engine.CharacterMovementComponent|GetMaxWalkSpeed (Variables|Character|GetCharacterMovement)) (* DeltaSeconds (* (Variables|Default|GetSlowMultiplier) (Math|Curves|GetFloatValue (Variables|Default|GetSpeedDecreaseRamp) (Math|Vector|VectorLength (Variables|/Script/Engine.MovementComponent|GetVelocity (Variables|Character|GetCharacterMovement))))))) 0.0)))
  (return _output_get))

(fn GetCurrentDistance
  (return (.x (Class|CharacterMovementComponent|GetLastUpdateLocation (Variables|/Script/Engine.Character|GetCharacterMovement (Game|GetPlayerCharacter 0))))))

(fn UpdateFlipbook
  ;[0.3057 0.2258 1] Set Status from IDLE to Run
  (Sprite|SetFlipbook (Variables|Default|GetSprite) (select (> (Math|Vector|VectorLength (Variables|/Script/Engine.MovementComponent|GetVelocity (Variables|Character|GetCharacterMovement))) 0.0) "/Game/PaperAssets/Runner/FB_Runner_Run.FB_Runner_Run" "/Game/PaperAssets/Runner/FB_Runner_IDLE.FB_Runner_IDLE")))

(fn SetRunPlayRate
  ;[0.4238 1 0.5256] CommentSpeed of the character movement
  (if (== (Class|PaperFlipbookComponent|GetFlipbook (Variables|Default|GetSprite)) "/Game/PaperAssets/Runner/FB_Runner_Run.FB_Runner_Run")
    (Components|Timeline|SetPlayRate (Variables|Default|GetSprite) (/ (Math|Vector|VectorLength (Variables|/Script/Engine.MovementComponent|GetVelocity (Variables|Character|GetCharacterMovement))) (Variables|Default|GetMaxSpeed)))
    (else
      (Components|Timeline|SetPlayRate (Variables|Default|GetSprite) 1.0))))

(fn StepsSound
  (bind _sprite (Variables|Default|GetSprite))
  (bind _returnvalue (Class|PaperFlipbookComponent|GetPlaybackPositioninFrames _sprite))
  (if (== (Class|PaperFlipbookComponent|GetFlipbook (Variables|Default|GetSprite)) "/Game/PaperAssets/Runner/FB_Runner_Run.FB_Runner_Run")
    (if (or (== _returnvalue 1) (== _returnvalue 5))
      (Audio|PlaySound2D "/Game/Sounds/Footsteps/S_Step_Concrete.S_Step_Concrete" 1.0 1.0 0.0 0 0))))